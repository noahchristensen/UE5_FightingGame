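; Player controller for the fighting game that creates and displays the match HUD.
; On BeginPlay, after a short delay, it adds a WBP_HUD widget to the viewport and hands it to the controlled fighter character.
; It then binds the HUD's two input-stack widgets to the characters of player 0 and player 1.
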(event `self.ReceiveBeginPlay`
  (`KismetSystemLibrary.Delay` 0.1)
  (bind _returnvalue (`|CreateWidget` "/Game/FightingGame/UI/WBP_HUD.WBP_HUD_C"))
  (`UserWidget.AddToViewport` _returnvalue 0)
  (bind _asbp_fighting_game_character (cast `/Game/FightingGame/Character/BP_FightingGameCharacter` (`self.K2_GetPawn`)))
  (set `/Game/FightingGame/Character/BP_FightingGameCharacter.HUD` _returnvalue _asbp_fighting_game_character)
  (bind _asfighting_game_character (cast `FightingGameCharacter` (`GameplayStatics.GetPlayerPawn` 0)))
  (set `/Game/FightingGame/UI/Input/WBP_InputStack.Character` _asfighting_game_character (`/Game/FightingGame/UI/WBP_HUD.WBP_InputStack` _returnvalue))
  (bind _asfighting_game_character_2 (cast `FightingGameCharacter` (`GameplayStatics.GetPlayerPawn` 1)))
  (set `/Game/FightingGame/UI/Input/WBP_InputStack.Character` _asfighting_game_character_2 (`/Game/FightingGame/UI/WBP_HUD.WBP_InputStack2` _returnvalue)))

(fn `UserConstructionScript`)