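; Fighting game character Blueprint that handles input buffer upkeep and on-screen input display.
; ShowInputonScreen sends each input name to one of two WBP_HUD input stacks, depending on whether the controller is player one's.
; UpdateInputs prunes buffered inputs older than a fraction of a second, then calls FinishAddToInputBuffer, so stale inputs are removed before command checks.
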(event `self.ShowInputOnScreen`
  (params (inputData :type "InputData Structure"))
  (if (== (`self.GetController`) (`GameplayStatics.GetPlayerController` 0))
    ;[1 1 1] Player 1 Inputs
    (bind _aswbp_hud (cast `/Game/FightingGame/UI/WBP_HUD` (`self.HUD`)))
    (`/Game/FightingGame/UI/Input/WBP_InputStack.Add Input` (`/Game/FightingGame/UI/WBP_HUD.WBP_InputStack` _aswbp_hud) inputData_inputName)
    (else
      ;[1 1 1] Player 2 Inputs
      (bind _aswbp_hud_2 (cast `/Game/FightingGame/UI/WBP_HUD` (`self.HUD`)))
      (`/Game/FightingGame/UI/Input/WBP_InputStack.Add Input` (`/Game/FightingGame/UI/WBP_HUD.WBP_InputStack2` _aswbp_hud_2) inputData_inputName))))

(event `self.UpdateInputs`
  (bind _inputbuffer (`self.InputBuffer`))
  ;[1 1 1] Make sure the For Loop runs properly
  (set `self.Array` _inputbuffer)
  (for _array_element (`self.Array`)
    ;[1 1 1] Remove inputs that are too old before trying to do Commands
    (if (< (`.timePassed` (break `InputData` _array_element)) (- (`GameplayStatics.GetTimeSeconds`) 0.4))
      (`KismetArrayLibrary.Array_RemoveItem` _inputbuffer _array_element)))
  (`self.FinishAddToInputBuffer`))

(fn `UserConstructionScript`)